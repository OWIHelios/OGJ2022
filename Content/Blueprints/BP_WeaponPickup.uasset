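; BP_WeaponPickup is a pickup actor that hands a weapon to the player character on overlap.
; Its construction script sets the static mesh from the WeaponData's weapon mesh, and Tick spins that mesh at RotationRate.
; When an actor enters the Box, it casts to BP_Character_Template and calls ChangeWeapon with WeaponData; the pickup is not destroyed afterwards.
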(event OnComponentBeginOverlap(Box)
  (params (OverlappedComponent :type Primitive%20Component%20Object%20Reference) (OtherActor :type Actor%20Object%20Reference) (OtherComp :type Primitive%20Component%20Object%20Reference) (OtherBodyIndex :type Integer) (bFromSweep :type Boolean) (SweepResult :type Hit%20Result%20Structure%20%28by%20ref%29))
  (bind _asbp_character_template (Utilities|Casting|CastToBP_Character_Template OtherActor))
  (Default|ChangeWeapon _asbp_character_template (Variables|Default|GetWeaponData)))

(event EventBeginPlay)

(event Collision|EventActorBeginOverlap
  (params (OtherActor :type Actor%20Object%20Reference)))

(event EventTick
  (params (DeltaSeconds :type Float%20%28single-precision%29))
  (Transformation|AddLocalRotation (Variables|Default|GetStaticMesh) (Math|Rotator|MakeRotator 0.0 0.0 (Variables|Default|GetRotationRate)) false false))

(fn ConstructionScript
  (Components|StaticMesh|SetStaticMesh (Variables|Default|GetStaticMesh) (.WeaponMesh (Utilities|Struct|BreakWeaponData (Variables|Default|GetWeaponData)))))