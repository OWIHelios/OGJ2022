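; Template game mode that tracks per-player points and names a victor against the game instance's GoalPoints.
; PostLogin registers each controller in the CurrentPoints map, and AddScore increments it, rebuilds a pipe-delimited PointsStr and sets VictorName on the goal check.
; EndGame, a separate event not triggered here, passes the victor, player names and points to player 0's character to create the scoreboard.
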(event Custom|EndGame
  (bind _asbp_character_template (Utilities|Casting|CastToBP_Character_Template (Pawn|GetControlledPawn (Game|GetPlayerController 0))))
  (bind _values (Utilities|Map|Values (Variables|Default|GetCurrentPoints)))
  (bind _names (CallFunction|GetFinalScores))
  (Default|CreateScoreboard _asbp_character_template (Variables|Default|GetVictorName) _names _values))

(event EventPostLogin
  (params (NewPlayer :type Player%20Controller%20Object%20Reference))
  (Utilities|Map|Add (Variables|Default|GetCurrentPoints) NewPlayer 0))

(fn ConstructionScript)

(fn RefreshScore
  (bind _values (Utilities|Map|Values (Variables|Default|GetCurrentPoints)))
  (for _array_element _values
    (LocalVariables|SetLOutput (select (Utilities|Array|IsEmpty (LocalVariables|GetLOutput)) (Utilities|String|ToString(Integer) _array_element) (Utilities|String|Append (LocalVariables|GetLOutput) " | " (Utilities|String|ToString(Integer) _array_element)))))
  (Variables|Default|SetPointsStr (LocalVariables|GetLOutput)))

(fn AddScore
  (params (Controller :type Controller%20Object%20Reference))
  (bind _currentpoints (Variables|Default|GetCurrentPoints))
  (bind _value (Utilities|Map|Find _currentpoints Controller))
  (bind _returnvalue (+ _value 1))
  (Utilities|Map|Add _currentpoints Controller _returnvalue)
  (bind _asbp_game_instance_template (Utilities|Casting|CastToBP_GameInstance_Template (Game|GetGameInstance)))
  (CallFunction|RefreshScore)
  (if (>= _returnvalue (Variables|/Game/Blueprints/Core/BP_GameInstance_Template.BP_GameInstance_Template_C|GetGoalPoints _asbp_game_instance_template))
    (Variables|Default|SetVictorName (PlayerState|GetPlayerName (Variables|/Script/Engine.Controller|GetPlayerState Controller)))))

(fn GetFinalScores
  (bind _keys (Utilities|Map|Keys (Variables|Default|GetCurrentPoints)))
  (for _array_element _keys
    (Utilities|Array|Add (LocalVariables|GetLNames) (PlayerState|GetPlayerName (Variables|/Script/Engine.Controller|GetPlayerState _array_element))))
  (return (LocalVariables|GetLNames)))